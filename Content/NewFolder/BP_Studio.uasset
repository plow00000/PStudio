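; BP_Studio is a Blueprint for a static mesh with a switchable emissive light.
; On BeginPlay it creates and stores a dynamic material instance for the mesh's "light" material slot.
; ToggleLight flips the LightOn flag and calls UpdateLight, which switches the material's EmissivePower parameter between on and off.
; UpdateLight is not called at BeginPlay, and a duplicate material-creation node is left unconnected.
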(event `self.ReceiveBeginPlay`
  (bind _staticmesh (`self.StaticMesh`))
  (bind _returnvalue (`PrimitiveComponent.CreateDynamicMaterialInstance` _staticmesh (`PrimitiveComponent.GetMaterialIndex` _staticmesh "light") (`PrimitiveComponent.GetMaterialByName` _staticmesh "light") "None"))
  (set `self.LightMatIns` _returnvalue))

(event `ToggleLight`
  (set `self.bLightOn` (not (`self.bLightOn`)))
  (`self.UpdateLight`))

(event `UpdateLight`
  (`MaterialInstanceDynamic.SetScalarParameterValue` (`self.LightMatIns`) "EmissivePower" (`KismetMathLibrary.SelectFloat` 1.0 0.0 (`self.bLightOn`))))

(fn `UserConstructionScript`)