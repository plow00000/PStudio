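; Player controller Blueprint that toggles a light UI widget on and off for the local player.
; On BeginPlay it adds the IMC_Default Enhanced Input mapping context and creates a WBP_Light widget without showing it.
; The IA_ToggleUI action value drives cursor visibility, adding the widget to the viewport with Game and UI input, or removing it and restoring game-only input.
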(event `self.ReceiveBeginPlay`
  (bind _returnvalue (subsystem `EnhancedInputLocalPlayerSubsystem`))
  (if (`self.IsLocalPlayerController`)
    (`/Engine/EditorBlueprintResources/StandardMacros.IsValid` _returnvalue
      (:`Is Valid`
        (`EnhancedInputSubsystemInterface.AddMappingContext` _returnvalue "/Game/NewFolder/IMC_Default.IMC_Default" 0 (struct))
        (bind _returnvalue_2 (`|CreateWidget` "/Game/NewFolder/WBP_Light.WBP_Light_C" self))
        (set `self.Widget` _returnvalue_2)))))

(event `EnhancedInput|/Game/NewFolder/IA_ToggleUI`
  (params (ActionValue :type Boolean) (ElapsedSeconds :type "Float (double-precision)") (TriggeredSeconds :type "Float (double-precision)") (InputAction :type "InputAction Object Reference" :default "/Game/NewFolder/IA_ToggleUI.IA_ToggleUI"))
  (:`Triggered`
    (bind _output_get (set `self.bShowMouseCursor` ActionValue))
    (if _output_get
      (`WidgetBlueprintLibrary.SetInputMode_GameAndUIEx` self null)
      (`UserWidget.AddToViewport` (`self.Widget`) 0)
      (else
        (`WidgetBlueprintLibrary.SetInputMode_GameOnly` self)
        (`Widget.RemoveFromParent` (`self.Widget`))))))

(fn `UserConstructionScript`)