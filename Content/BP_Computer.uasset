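; Interactable in-world computer that lets the player use a browser UI on its screen.
; Overlap registers it as the player pawn's interactor and toggles a "Press F" prompt.
; Interact freezes the pawn, saves and moves its follow camera to face the panel, then shows the screen widget with UI-only mouse input.
; World and screen components share one browser widget; ReleaseUser only hides the screen component.
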(event `self.ReceiveBeginPlay`
  (bind _worldwidget (`self.WorldWidget`))
  (bind _screenwidget (`self.ScreenWidget`))
  (`WidgetComponent.SetWidget` _worldwidget (`WidgetComponent.GetWidget` _screenwidget))
  (`WidgetComponent.SetDrawSize` _worldwidget (`WidgetComponent.GetDrawSize` _screenwidget))
  (`SceneComponent.K2_SetRelativeTransform` (`self.ScreenWidget`) (`SceneComponent.GetRelativeTransform` (`self.WorldWidget`)) false false))

(event `self.ReceiveActorBeginOverlap`
  (params (OtherActor :type "Actor Object Reference"))
  (bind _pressfwidget (`self.PressFWidget`))
  (if (== OtherActor (`Controller.K2_GetPawn` (`GameplayStatics.GetPlayerController` 0)))
    (bind _asbp_player_pawn (cast `/Game/Framework/BP_PlayerPawn` OtherActor))
    (`/Game/Framework/BP_PlayerPawn.SetInteractor` _asbp_player_pawn self)
    (`SceneComponent.SetVisibility` _pressfwidget true false)
    (`SceneComponent.K2_SetWorldRotation` _pressfwidget (`KismetMathLibrary.FindLookAtRotation` (`SceneComponent.K2_GetComponentLocation` _pressfwidget) (`self.K2_GetActorLocation`)) false false)))

(event `self.ReceiveActorEndOverlap`
  (params (OtherActor :type "Actor Object Reference"))
  (if (== OtherActor (`Controller.K2_GetPawn` (`GameplayStatics.GetPlayerController` 0)))
    (bind _asbp_player_pawn (cast `/Game/Framework/BP_PlayerPawn` OtherActor))
    (`/Game/Framework/BP_PlayerPawn.SetInteractor` _asbp_player_pawn null)
    (`SceneComponent.SetVisibility` (`self.PressFWidget`) false false)))

(event `/Game/BPI_Interaction.Interact`
  (bind _returnvalue (`GameplayStatics.GetPlayerController` 0))
  (bind _panel (`self.Panel`))
  (bind _returnvalue_2 (`SceneComponent.K2_GetComponentLocation` _panel))
  (bind _returnvalue_3 (+ (* 30.0 (`SceneComponent.GetUpVector` _panel)) _returnvalue_2))
  (bind _asbp_player_pawn (cast `/Game/Framework/BP_PlayerPawn` (`Controller.K2_GetPawn` (`GameplayStatics.GetPlayerController` 0))))
  (`/Game/Framework/BP_PlayerPawn.SetInteractor` _asbp_player_pawn null)
  (set `/Game/Framework/BP_PlayerPawn.Movable` false _asbp_player_pawn)
  (`MovementComponent.StopMovementImmediately` (`Character.CharacterMovement` _asbp_player_pawn))
  (bind _followcamera (`/Game/Framework/BP_PlayerPawn.FollowCamera` _asbp_player_pawn))
  (set `self.CameraTransform` (`SceneComponent.K2_GetComponentToWorld` _followcamera))
  (`SceneComponent.K2_SetWorldLocationAndRotation` _followcamera _returnvalue_3 (`KismetMathLibrary.FindLookAtRotation` _returnvalue_3 _returnvalue_2) false false)
  (`SceneComponent.SetVisibility` (`self.PressFWidget`) false false)
  (bind _aswbp_computer_browser (cast `/Game/WBP_ComputerBrowser` (`WidgetComponent.GetWidget` (`self.WorldWidget`))))
  (set `/Game/WBP_ComputerBrowser.OwnerComputer` self _aswbp_computer_browser)
  (set `PlayerController.bShowMouseCursor` true _returnvalue)
  (`WidgetBlueprintLibrary.SetInputMode_UIOnlyEx` _returnvalue (`WidgetComponent.GetWidget` (`self.ScreenWidget`)))
  (`SceneComponent.SetVisibility` (`self.ScreenWidget`) true false)
  (`KismetSystemLibrary.PrintString` "Visible"))

(fn `ReleaseUser`
  (`SceneComponent.SetVisibility` (`self.ScreenWidget`) false false))

(fn `UserConstructionScript`)