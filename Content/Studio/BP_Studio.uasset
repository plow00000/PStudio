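; BP_Studio is the studio environment actor that switches its lighting on or off by zone: master, indoor, salon, office or outside.
; On BeginPlay it creates dynamic materials for the mesh's lamp and two exterior slots, found by name.
; ToggleLight finds each zone's light Blueprint via GetActorOfClass and forwards the state.
; Office and outside toggles also set emissive power on the lamp and exterior materials respectively.
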(event `self.ReceiveBeginPlay`
  (bind _staticmesh (`self.StaticMesh`))
  (bind _staticmesh_2 (`self.StaticMesh`))
  (bind _staticmesh_3 (`self.StaticMesh`))
  (bind _returnvalue (`PrimitiveComponent.CreateDynamicMaterialInstance` _staticmesh (`PrimitiveComponent.GetMaterialIndex` _staticmesh "light") (`PrimitiveComponent.GetMaterialByName` _staticmesh "light") "None"))
  (set `self.LightMatIns` _returnvalue)
  (`|ExecutionSequence`
    (:`then_0`
      (bind _returnvalue_2 (`PrimitiveComponent.CreateDynamicMaterialInstance` _staticmesh_3 (`PrimitiveComponent.GetMaterialIndex` _staticmesh_3 "exterior0") (`PrimitiveComponent.GetMaterialByName` _staticmesh_3 "exterior0") "None"))
      (`KismetArrayLibrary.Array_Add` (`self.Exteriors`) _returnvalue_2))
    (:`then_1`
      (bind _returnvalue_3 (`PrimitiveComponent.CreateDynamicMaterialInstance` _staticmesh_2 (`PrimitiveComponent.GetMaterialIndex` _staticmesh_2 "exterior1") (`PrimitiveComponent.GetMaterialByName` _staticmesh_2 "exterior1") "None"))
      (`KismetArrayLibrary.Array_Add` (`self.Exteriors`) _returnvalue_3))))

(event `ToggleLamp`
  (params (IsOn :type Boolean))
  (bind _lightmatins (`self.LightMatIns`)
    (:`then`
      (`MaterialInstanceDynamic.SetScalarParameterValue` _lightmatins "EmissivePower" (`KismetMathLibrary.SelectFloat` 1.0 0.0 IsOn)))
    (:`else`)))

(event `ToggleNatLight`
  (params (IsOn :type Boolean))
  (for _array_element (`self.Exteriors`)
    (`MaterialInstanceDynamic.SetScalarParameterValue` _array_element "EmissivePower" (`KismetMathLibrary.SelectFloat` 1.0 0.0 IsOn))))

(fn `ToggleLight`
  (params (Selection :type "/Game/Studio/EN_Room Enum" :default "NewEnumerator0") (IsOn :type Boolean))
  (switch `/Game/Studio/EN_Room` Selection
    (:`NewEnumerator0`
      (`|ExecutionSequence`
        (:`then_0`
          (`|ExecutionSequence` :!label _label
            (:`then_0`
              (bind _returnvalue (`GameplayStatics.GetActorOfClass` "/Game/Studio/BP_SalonLight.BP_SalonLight_C" :!label _label_2))
              (`/Engine/EditorBlueprintResources/StandardMacros.IsValid` _returnvalue
                (:`Is Valid`
                  (`/Game/Studio/BP_SalonLight.ToggleLight` _returnvalue (`local.IsOn`)))))
            (:`then_1`
              (bind _returnvalue_2 (`GameplayStatics.GetActorOfClass` "/Game/Studio/BP_OfficeLight.BP_OfficeLight_C" :!label _label_3))
              (`/Engine/EditorBlueprintResources/StandardMacros.IsValid` _returnvalue_2
                (:`Is Valid`
                  (`/Game/Studio/BP_OfficeLight.ToggleLight` _returnvalue_2 (`local.IsOn`))
                  (`self.ToggleLamp` (`local.IsOn`)))))))
        (:`then_1`
          (bind _returnvalue_3 (`GameplayStatics.GetActorOfClass` "/Game/Studio/BP_OutsideLight.BP_OutsideLight_C" :!label _label_4))
          (`/Engine/EditorBlueprintResources/StandardMacros.IsValid` _returnvalue_3
            (:`Is Valid`
              (`/Game/Studio/BP_OutsideLight.ToggleLight` _returnvalue_3 (`local.IsOn`))
              (`self.ToggleNatLight` (`local.IsOn`)))))))
    (:`NewEnumerator1`
      (goto _label))
    (:`NewEnumerator2`
      (goto _label_2))
    (:`NewEnumerator3`
      (goto _label_3))
    (:`NewEnumerator4`
      (goto _label_4))))

(fn `UserConstructionScript`)