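; BP_Computer is an interactable computer actor that opens a browser UI, which it also sets as the source for its Projectors.
; Overlap registers it as the player pawn's interactor and toggles a "Press F" prompt.
; A server interaction claims it through IsUsed and relays to the client, which shows the browser, freezes movement, switches view and enables UI-only input.
; InteractStop clears the flag, while ReleaseUser restores pawn movement.
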(event `self.ReceiveBeginPlay`
  (bind _returnvalue (`|CreateWidget` "/Game/Blueprint/Computer/WBP_ComputerBrowser.WBP_ComputerBrowser_C" null self))
  (set `self.BrowserWidget` _returnvalue)
  (for _array_element (`self.Projectors`)
    (`/Game/BP_Projector.SetSource` _array_element (`self.BrowserWidget`))))

(event `self.ReceiveActorBeginOverlap`
  (params (OtherActor :type "Actor Object Reference"))
  (bind _pressfwidget (`self.PressFWidget`))
  (bind _asbp_player_pawn (cast `/Game/Framework/BP_PlayerPawn` OtherActor))
  (`/Game/Framework/BP_PlayerPawn.SetInteractor` _asbp_player_pawn self)
  (`SceneComponent.SetVisibility` _pressfwidget true false)
  (`SceneComponent.K2_SetWorldRotation` _pressfwidget (`KismetMathLibrary.FindLookAtRotation` (`SceneComponent.K2_GetComponentLocation` _pressfwidget) (`self.K2_GetActorLocation`)) false false))

(event `self.ReceiveActorEndOverlap`
  (params (OtherActor :type "Actor Object Reference"))
  (bind _asbp_player_pawn (cast `/Game/Framework/BP_PlayerPawn` OtherActor))
  (`/Game/Framework/BP_PlayerPawn.SetInteractor` _asbp_player_pawn null)
  (`SceneComponent.SetVisibility` (`self.PressFWidget`) false false))

(event `/Game/BPI_Interaction.InteractOnServer`
  (params (PC :type "/Game/Framework/BP_PC Object Reference"))
  (if (not (`self.bIsUsed`))
    (set `self.bIsUsed` true)
    (`/Game/Framework/BP_PC.S2C_Interact` PC self)))

(event `/Game/BPI_Interaction.InteractOnClient`
  (params (PC :type "/Game/Framework/BP_PC Object Reference"))
  (set `self.PC` PC)
  (`self.FuncInteract`))

(event `/Game/BPI_Interaction.InteractStop`
  (set `self.bIsUsed` false))

(fn `FuncInteract`
  (bind _pc (`self.PC`))
  (bind _pc_2 (`self.PC`))
  (bind _browserwidget (`self.BrowserWidget`)
    (:`then`
      (`UserWidget.AddToViewport` _browserwidget 0)
      (set `self.bWidgetVisible` true)
      (if (`Controller.IsLocalPlayerController` _pc_2)
        (bind _asbp_player_pawn (cast `/Game/Framework/BP_PlayerPawn` (`Controller.K2_GetPawn` _pc_2)))
        (`/Game/Framework/BP_PlayerPawn.SetInteractor` _asbp_player_pawn self)
        (set `/Game/Framework/BP_PlayerPawn.Movable` false _asbp_player_pawn)
        (`MovementComponent.StopMovementImmediately` (`Character.CharacterMovement` _asbp_player_pawn))
        (`PlayerController.SetViewTargetWithBlend` (`self.PC`) self 0.0 "VTBlend_Linear" 0.0 false)
        (`SceneComponent.SetVisibility` (`self.PressFWidget`) false false)
        (set `PlayerController.bShowMouseCursor` true _pc)
        (`WidgetBlueprintLibrary.SetInputMode_UIOnlyEx` _pc (`self.BrowserWidget`))))
    (:`else`)))

(fn `ReleaseUser`
  (bind _pc (`self.PC`))
  (set `/Game/Framework/BP_PC.OnInteraction` false _pc)
  (bind _asbp_player_pawn (cast `/Game/Framework/BP_PlayerPawn` (`Controller.K2_GetPawn` _pc)))
  (set `/Game/Framework/BP_PlayerPawn.Movable` true _asbp_player_pawn))

(fn `UserConstructionScript`)