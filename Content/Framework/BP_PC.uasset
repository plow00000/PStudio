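; Player controller for a networked game that handles interaction, a toggleable light-control widget and shared control of a BP_Computer web browser.
; Input sets up Enhanced Input and the UI mode, while named client/server events route interact and stop calls to Interactor objects.
; URL changes and JavaScript are relayed through every controller in the PlayerArray to the first BP_Computer found.
; The M key toggles the view to the nearest BP_Projector and locks pawn movement.
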(event `self.ReceiveBeginPlay`
  (bind _returnvalue (subsystem `EnhancedInputLocalPlayerSubsystem`))
  (if (`self.IsLocalPlayerController`)
    (`/Engine/EditorBlueprintResources/StandardMacros.IsValid` _returnvalue
      (:`Is Valid`
        (`EnhancedInputSubsystemInterface.AddMappingContext` _returnvalue "/Game/Input/IMC_Default.IMC_Default" 0 (struct))
        (bind _returnvalue_2 (`|CreateWidget` "/Game/Framework/WBP_Light.WBP_Light_C" self))
        (set `self.Widget` _returnvalue_2)))))

(event `EnhancedInput|/Game/Input/IA_ToggleUI`
  (params (ActionValue :type Boolean) (ElapsedSeconds :type "Float (double-precision)") (TriggeredSeconds :type "Float (double-precision)") (InputAction :type "InputAction Object Reference" :default "/Game/Input/IA_ToggleUI.IA_ToggleUI"))
  (:`Triggered`
    (if (not (`self.OnInteraction`))
      (bind _output_get (set `self.IsLightControlOn` ActionValue))
      (if _output_get
        (`WidgetBlueprintLibrary.SetInputMode_GameAndUIEx` self (`self.Widget`))
        (`UserWidget.AddToViewport` (`self.Widget`) 0)
        (set `self.bShowMouseCursor` true)
        (else
          (`WidgetBlueprintLibrary.SetInputMode_GameOnly` self)
          (`Widget.RemoveFromParent` (`self.Widget`))
          (set `self.bShowMouseCursor` false))))))

(event `EnhancedInput|/Game/Input/Actions/IA_Interact`
  (params (ActionValue :type Boolean) (ElapsedSeconds :type "Float (double-precision)") (TriggeredSeconds :type "Float (double-precision)") (InputAction :type "InputAction Object Reference" :default "/Game/Input/Actions/IA_Interact.IA_Interact"))
  (:`Started`
    (`self.C2S_Interact`)))

(event `C2S_Interact`
  ; Interaction
  (message `/Game/BPI_Interaction.InteractOnServer` (`self.Interactor`) self))

(event `C2S_StopIneteract`
  (params (Interactor :type "/Game/BPI_Interaction Interface"))
  ; Interaction
  (`self.S2A_StopInteract` Interactor))

(event `S2C_Interact`
  (params (Interactor :type "/Game/BPI_Interaction Interface"))
  ; Interaction
  (`self.Interact` Interactor))

(event `S2A_StopInteract`
  (params (Interactor :type "/Game/BPI_Interaction Interface"))
  ; Interaction
  (`/Game/BPI_Interaction.InteractStop` Interactor))

(event `Interact`
  (params (Interactor :type "/Game/BPI_Interaction Interface"))
  ; Interaction
  (`/Game/BPI_Interaction.InteractOnClient` Interactor self)
  (`KismetSystemLibrary.PrintString` (`KismetSystemLibrary.GetDisplayName` self)))

(event `C2S_ChangeURL`
  (params (Computer :type "/Game/Blueprint/Computer/BP_Computer Object Reference") (InURL :type String))
  ; Address Control
  (`self.S2A_ChangeURL` Computer InURL))

(event `ChangeURL`
  (params (Computer :type "/Game/Blueprint/Computer/BP_Computer Object Reference") (NewURL :type String))
  ; Address Control
  (bind _returnvalue (`GameplayStatics.GetActorOfClass` "/Game/Blueprint/Computer/BP_Computer.BP_Computer_C"))
  (`KismetSystemLibrary.PrintString` "Called" true true (struct :`G` 0.66 :`B` 1.0 :`A` 1.0) 20.0)
  (bind _webbrowser (`/Game/Blueprint/Computer/WBP_ComputerBrowser.WebBrowser` (`/Game/Blueprint/Computer/BP_Computer.BrowserWidget` _returnvalue)))
  (`WebBrowser.LoadURL` _webbrowser NewURL)
  (`Widget.SetFocus` _webbrowser))

(event `S2A_ChangeURL`
  (params (Computer :type "/Game/Blueprint/Computer/BP_Computer Object Reference") (InURL :type String))
  ; Address Control
  (for _array_element (`GameStateBase.PlayerArray` (`GameplayStatics.GetGameState`))
    (bind _asbp_pc (cast `/Game/Framework/BP_PC` (`PlayerState.GetPlayerController` _array_element)))
    (bind _returnvalue (`GameplayStatics.GetActorOfClass` "/Game/Blueprint/Computer/BP_Computer.BP_Computer_C"))
    (if (!= (`/Game/Blueprint/Computer/BP_Computer.PC` _returnvalue) self)
      (`self.ChangeURL` _asbp_pc _returnvalue InURL))))

(event `C2S_SendJS`
  (params (JS :type String))
  (for _array_element (`GameStateBase.PlayerArray` (`GameplayStatics.GetGameState`))
    (bind _asbp_pc (cast `/Game/Framework/BP_PC` (`PlayerState.GetPlayerController` _array_element)))
    (`self.RecieveJS` _asbp_pc JS)))

(event `RecieveJS`
  (params (JS :type String))
  (bind _returnvalue (`GameplayStatics.GetActorOfClass` "/Game/Blueprint/Computer/BP_Computer.BP_Computer_C"))
  (`WebBrowser.ExecuteJavascript` (`/Game/Blueprint/Computer/WBP_ComputerBrowser.WebBrowser` (`/Game/Blueprint/Computer/BP_Computer.BrowserWidget` _returnvalue)) JS))

(event `Key|M`
  (params (Key :type "Key Structure"))
  (:`Pressed`
    (set `self.IsViewing` (not (`self.IsViewing`)))
    (bind _outactors (`GameplayStatics.GetAllActorsOfClass` "/Game/BP_Projector.BP_Projector_C"))
    (`self.SetViewTargetWithBlend` (select `bool` (`self.IsViewing`) :`false` self :`true` (`.ReturnValue` (`GameplayStatics.FindNearestActor` (`self.K2_GetActorLocation` (`self.K2_GetPawn`)) _outactors)) :!type "Actor Object Reference"))
    (bind _asbp_player_pawn (cast `/Game/Framework/BP_PlayerPawn` (`self.K2_GetPawn`)))
    (set `/Game/Framework/BP_PlayerPawn.Movable` (not (`self.IsViewing`)) _asbp_player_pawn)))

(fn `UserConstructionScript`)